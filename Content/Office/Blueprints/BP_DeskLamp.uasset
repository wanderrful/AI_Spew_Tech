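; BP_DeskLamp is an office desk lamp that switches on and off when used.
; The OnUse event plays a sound, flips IsOn and calls Enable or Disable, and BeginPlay calls Disable so the lamp starts dark.
; Both events set the SpotLight's intensity and also toggle its shadow casting, so an unlit lamp casts no shadows.
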(event `self.ReceiveBeginPlay`
  (`self.Disable`))

(event `self.OnUse`
  (`AudioComponent.Play` (`self.Audio`) 0.0)
  (bind _output_get (set `self.IsOn` (not (`self.IsOn`))))
  (if _output_get
    (`self.Enable`)
    (else
      (`self.Disable`))))

(event `Enable`
  (bind _spotlight (`self.SpotLight`))
  (`LightComponentBase.SetCastShadows` _spotlight true)
  (`LightComponent.SetIntensity` _spotlight 5000.0))

(event `Disable`
  (bind _spotlight (`self.SpotLight`))
  (`LightComponentBase.SetCastShadows` _spotlight false)
  (`LightComponent.SetIntensity` _spotlight 0.0))

(fn `UserConstructionScript`)