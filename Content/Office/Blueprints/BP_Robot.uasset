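; BP_Robot is the office robot that voices the tutorial, nags and zaps the player, and scolds them when performance runs out.
; Voice, wait and movement calls chain through delegate events, with counters escalating reminders and wrong-answer responses from warnings to zaps.
; A correct tutorial answer starts the performance decrease and sends the robot to the corridor end.
; Helper events drive arm and face animations, and Tick can turn the mesh toward the player camera.
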(event `eh_OnExtendArm`
  (bind _asabp_robot_arm (cast `/Game/Office/Characters/ABP_RobotArm` (`SkeletalMeshComponent.GetAnimInstance` (`self.Arm`))))
  (`/Game/Office/Characters/ABP_RobotArm.eh_OnExtendArm` _asabp_robot_arm))

(event `eh_OnRetractArm`
  (bind _asabp_robot_arm (cast `/Game/Office/Characters/ABP_RobotArm` (`SkeletalMeshComponent.GetAnimInstance` (`self.Arm`))))
  (`/Game/Office/Characters/ABP_RobotArm.eh_OnRetractArm` _asabp_robot_arm))

(event `eh_OnBlink`
  (bind _asabp_robot_manager (cast `/Game/Office/Characters/ABP_RobotManager` (`SkeletalMeshComponent.GetAnimInstance` (`self.Mesh`))))
  (`/Game/Office/Characters/ABP_RobotManager.eh_OnBlink` _asabp_robot_manager))

(event `eh_OnTwitchEye`
  (bind _asabp_robot_manager (cast `/Game/Office/Characters/ABP_RobotManager` (`SkeletalMeshComponent.GetAnimInstance` (`self.Mesh`))))
  (`/Game/Office/Characters/ABP_RobotManager.eh_OnEyeTwitch` _asabp_robot_manager))

(event `lmkkjmp;`)

(event `self.OnStartTutorial`
  (set `self.Tutorial` true)
  (`OfficeStatics.RobotPlayVoice` "/Game/Sounds/SamVoiceLines/Sam_Tutorial1.Sam_Tutorial1" (delegate `CustomEvent_1`)))

(event `NotifyPressButton`
  (if (`self.Safty`)
    (`OfficeStatics.RobotPlayVoice` null (delegate `NotifyPressButton`))
    (else
      (`OfficeStatics.RobotPlayVoice` "/Game/Sounds/SamVoiceLines/Sam_TutorialSkippedSafty.Sam_TutorialSkippedSafty" (delegate `CustomEvent_0`)))))

(event `CustomEvent_1`
  (`OfficeStatics.RobotPlayVoice` "/Game/Sounds/SamVoiceLines/Sam_Tutorial2.Sam_Tutorial2" (delegate `CustomEvent_2`)))

(event `NotifyCAPTCHAStart`
  (`OfficeStatics.RobotPlayVoice` "/Game/Sounds/SamVoiceLines/Sam_Tutorial4.Sam_Tutorial4" (delegate `Anotherevent`)))

(event `NotifyGoodAnwser`
  (if (`self.Tutorial`)
    (set `self.Tutorial` false)
    (`OfficeStatics.RobotPlayVoice` "/Game/Sounds/SamVoiceLines/Sam_Tutorial5.Sam_Tutorial5" (delegate `CustomEvent_4`))
    (elif (`self.bItsZapTime`)
      (if (`self.bool`)
        (`OfficeStatics.RobotPlayVoice` "/Game/Sounds/SamVoiceLines/Sam_Ok.Sam_Ok" (delegate `lmkkjmp;`))
        (`OfficeStatics.RobotGoTo` "FrontCorridorEnd" :!label _label)
        (set `self.bItsZapTime` false)))))

(event `CustomEvent_0`)

(event `CustomEvent_2`
  (set `self.Safty` true)
  (`OfficeStatics.RobotPlayVoice` "/Game/Sounds/SamVoiceLines/Sam_Tutorial3.Sam_Tutorial3" (delegate `CustomEvent_3`)))

(event `Anotherevent`
  (`self.Wait` 10.0 (delegate `fdgdfgdf`)))

(event `CustomEvent_4`
  (`OfficeGameMode.StartPerforamceDescrese` (`OfficeStatics.GetOfficeGameMode`))
  (`OfficeStatics.RobotPlayVoice` "/Game/Sounds/SamVoiceLines/Sam_Tutorial6.Sam_Tutorial6" (delegate `fgdsfgdfghdjh`)))

(event `self.OnZap`
  (`GameplayStatics.PlaySound2D` "/Game/Sounds/ShortSounds/Zap_Cue.Zap_Cue" 1.0 1.0 0.0 null null))

(event `CustomEvent_3`
  (`OfficeStatics.RobotWait` 10.0 (delegate `jnjnj`)))

(event `fgdsfgdfghdjh`
  (`OfficeStatics.RobotGoTo` "FrontCorridorEnd"))

(event `NotifyBadAnwser`
  (bind _tutorialbadanwsers (`self.TutorialBadAnwsers`))
  (if (`self.Tutorial`)
    (switch `int` _tutorialbadanwsers
      (:`0`
        (`self.PlayVoiceWithoutDelegate` "/Game/Sounds/SamVoiceLines/Sam_TutorialTypeWrong1.Sam_TutorialTypeWrong1"))
      (:`1`
        (`self.PlayVoiceWithoutDelegate` "/Game/Sounds/SamVoiceLines/Sam_TutorialTypeWrong2.Sam_TutorialTypeWrong2"))
      (:`2`
        (`self.PlayVoiceWithoutDelegate` "/Game/Sounds/SamVoiceLines/Sam_TutorialTypeWrong3.Sam_TutorialTypeWrong3"))
      (:`3`
        (`self.PlayVoiceWithoutDelegate` "/Game/Sounds/SamVoiceLines/Sam_TutorialTypeWrongZap1.Sam_TutorialTypeWrongZap1")
        (`self.Zap`))
      (:`4`
        (`self.PlayVoiceWithoutDelegate` "/Game/Sounds/SamVoiceLines/Sam_TutorialTypeWrongZap2.Sam_TutorialTypeWrongZap2")
        (`self.Zap`))
      (:`5`
        (`self.PlayVoiceWithoutDelegate` "/Game/Sounds/SamVoiceLines/Sam_TutorialTypeWrongZap3.Sam_TutorialTypeWrongZap3")
        (`self.Zap`)))
    (`/Engine/EditorBlueprintResources/StandardMacros.IncrementInt` _tutorialbadanwsers
      (:`  `
        (`self.Wait` 10.0 (delegate `fdgdfgdf`) :!label _label_2)
        (`/Engine/EditorBlueprintResources/StandardMacros.IncrementInt` (`self.CountType`))))))

(event `fdgdfgdf`
  (switch `int` (`self.CountType`)
    (:`0`
      (`self.PlayVoiceWithoutDelegate` "/Game/Sounds/SamVoiceLines/Sam_TutorialTypeWait1.Sam_TutorialTypeWait1")
      (goto _label_2))
    (:`1`
      (`self.PlayVoiceWithoutDelegate` "/Game/Sounds/SamVoiceLines/Sam_TutorialTypeWait2.Sam_TutorialTypeWait2")
      (goto _label_2))
    (:`2`
      (`self.PlayVoiceWithoutDelegate` "/Game/Sounds/SamVoiceLines/Sam_TutorialTypeWait3.Sam_TutorialTypeWait3")
      (goto _label_2))
    (:`3`
      (`self.PlayVoiceWithoutDelegate` "/Game/Sounds/SamVoiceLines/Sam_TutorialTypeZap1.Sam_TutorialTypeZap1")
      (`self.Zap`)
      (goto _label_2))
    (:`4`
      (`self.PlayVoiceWithoutDelegate` "/Game/Sounds/SamVoiceLines/Sam_TutorialTypeZap2.Sam_TutorialTypeZap2")
      (`self.Zap`)
      (goto _label_2))
    (:`5`
      (`self.PlayVoiceWithoutDelegate` "/Game/Sounds/SamVoiceLines/Sam_TutorialTypeZap3.Sam_TutorialTypeZap3")
      (`self.Zap`)
      (goto _label_2))))

(event `self.OnAboutToZap`
  (`OfficeStatics.RobotPlayVoice` "/Game/Sounds/SamVoiceLines/Sam_Zap1.Sam_Zap1" (delegate `NONONONO`))
  (`self.Zap`)
  (if (not (> (`OfficeGameMode.Performance` (`OfficeStatics.GetOfficeGameMode`)) 0.0))
    (`self.Wait` 15.0 (delegate `You so dead`))
    (set `self.bool` true :!label _label_3)))

(event `jnjnj`
  (bind _countbutton (`self.CountButton`))
  (switch `int` _countbutton
    (:`0`
      (`self.PlayVoiceWithoutDelegate` "/Game/Sounds/SamVoiceLines/Sam_TutorialButtonWait1.Sam_TutorialButtonWait1"))
    (:`1`
      (`self.PlayVoiceWithoutDelegate` "/Game/Sounds/SamVoiceLines/Sam_TutorialButtonWait2.Sam_TutorialButtonWait2"))
    (:`2`
      (`self.PlayVoiceWithoutDelegate` "/Game/Sounds/SamVoiceLines/Sam_TutorialButtonWait3.Sam_TutorialButtonWait3"))
    (:`3`
      (`self.PlayVoiceWithoutDelegate` "/Game/Sounds/SamVoiceLines/Sam_TutorialButtonZap1.Sam_TutorialButtonZap1")
      (`self.Zap`))
    (:`4`
      (`self.PlayVoiceWithoutDelegate` "/Game/Sounds/SamVoiceLines/Sam_TutorialButtonZap2.Sam_TutorialButtonZap2")
      (`self.Zap`))
    (:`5`
      (`self.PlayVoiceWithoutDelegate` "/Game/Sounds/SamVoiceLines/Sam_TutorialButtonZap3.Sam_TutorialButtonZap3")
      (`self.Zap`)))
  (`self.Wait` 10.0 (delegate `jnjnj`))
  (`/Engine/EditorBlueprintResources/StandardMacros.IncrementInt` _countbutton))

(event `NONONONO`
  (if (> (`OfficeGameMode.Performance` (`OfficeStatics.GetOfficeGameMode`)) 0.0)
    (goto _label)
    (else
      (goto _label_3))))

(event `You so dead`
  (`OfficeStatics.RobotPlayVoice` "/Game/Sounds/SamVoiceLines/Sam_GetBackToWork1.Sam_GetBackToWork1" (delegate `CustomEvent_5`))
  (`self.Zap`))

(event `CustomEvent_5`
  (`self.Wait` 10.0 (delegate `CustomEvent`)))

(event `CustomEvent`
  (`OfficeStatics.RobotPlayVoice` "/Game/Sounds/SamVoiceLines/Sam_GetBackToWork2.Sam_GetBackToWork2" (delegate `CustomEvent_6`))
  (`self.Zap`))

(event `CustomEvent_6`)

(event `eh_OnLookAtPlayer`
  (params (bShouldLook :type Boolean))
  (set `self.bShouldLookAtPlayer` bShouldLook))

(event `self.ReceiveTick`
  (params (DeltaSeconds :type "Float (single-precision)"))
  (bind _returnvalue (`GameplayStatics.GetPlayerCameraManager` 0))
  (`/Engine/EditorBlueprintResources/StandardMacros.IsValid` _returnvalue
    (:`Is Valid`
      (if (`self.bShouldLookAtPlayer`)
        (`SceneComponent.K2_SetWorldRotation` (`self.Mesh`) (`KismetMathLibrary.FindLookAtRotation` (`SceneComponent.K2_GetComponentLocation` (`self.Mesh`)) (`self.GetActorEyesViewPoint` _returnvalue)) false false)))))

(fn `UserConstructionScript`
  (`SceneComponent.K2_AttachToComponent` (`self.Arm`) (`self.Mesh`) "ArmSocket" "SnapToTarget" "SnapToTarget" "SnapToTarget" true))