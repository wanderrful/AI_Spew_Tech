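; BP_PneumaticPost is an office pneumatic post actor with a physics-constrained door and a lock status lamp.
; LockDoor locks the constraint's swing, resets the door's rotation and turns the lamp red.
; UnlockDoor limits swing to the angle read from the constraint's current swing at BeginPlay, turns the lamp green and plays an air-release sound.
; BeginPlay calls LockDoor and then immediately UnlockDoor, so the door starts unlocked.
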(event `self.ReceiveBeginPlay`
  (set `self.ConstraintAngle` (`PhysicsConstraintComponent.GetCurrentSwing1` (`self.DoorConstraint`)))
  (`self.LockDoor`)
  (`self.UnlockDoor`))

(event `LockDoor`
  (`PhysicsConstraintComponent.SetAngularSwing1Limit` (`self.DoorConstraint`) "ACM_Locked" 0.0)
  (`SceneComponent.K2_SetRelativeRotation` (`self.Door`) (struct :`Yaw` 90.0) false false)
  (`PrimitiveComponent.SetMaterial` (`self.Lamp`) 0 "/Game/Office/Materials/MI_RedLamp.MI_RedLamp"))

(event `UnlockDoor`
  (`PhysicsConstraintComponent.SetAngularSwing1Limit` (`self.DoorConstraint`) "ACM_Limited" (`self.ConstraintAngle`))
  (`PrimitiveComponent.SetMaterial` (`self.Lamp`) 0 "/Game/Office/Materials/MI_GreenLamp.MI_GreenLamp")
  (`AudioComponent.SetSound` (`self.Audio`) "/Game/Sounds/Unsort/Slips_Air_Release_01.Slips_Air_Release_01")
  (`AudioComponent.Play` (`self.Audio`) 0.0))

(fn `UserConstructionScript`)