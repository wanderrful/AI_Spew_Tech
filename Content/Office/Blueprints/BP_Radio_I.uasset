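; BP_Radio_I is a usable office radio that cycles through a music loop, radio noise and an empty sound slot.
; Using it plays a click, waits briefly, clears any pending Morse timer and plays the next entry on a single Audio component.
; Tuning to the noise arms a 60-second timer that swaps in a Morse code cue.
; An intro transition event starts the first track at a given time offset.
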(event `self.ReceiveBeginPlay`
  (set `self.SongsList` (`|MakeArray` "/Game/Sounds/Music/A_Stratosphere_Loop.A_Stratosphere_Loop" "/Game/Sounds/Music/A_Radio_Noise.A_Radio_Noise" null :!type "SoundWave Object Reference")))

(event `TransitFromIntrol`
  (params (StartTime :type "Float (double-precision)"))
  (set `self.CurrentSongIndex` 0)
  (`self.PlaySong` StartTime))

(event `Click`
  (bind _audio (`self.Audio`))
  (set `AudioComponent.Sound` "/Game/Sounds/Unsort/Click.Click" _audio)
  (`AudioComponent.Play` _audio 0.0))

(event `self.OnUse`
  (`self.Click`)
  (`KismetSystemLibrary.Delay` 0.2)
  (`KismetSystemLibrary.K2_ClearTimer` null "MorzeSignal")
  (`self.PlaySong` 0.0))

(event `PlaySong`
  (params (StartTime :type "Float (double-precision)"))
  (bind _audio (`self.Audio`))
  (bind _songslist (`self.SongsList`))
  (bind _currentsongindex (`self.CurrentSongIndex`))
  (set `AudioComponent.Sound` (`|GetArrayItem` _songslist _currentsongindex) _audio)
  (`AudioComponent.Play` _audio StartTime)
  (if (== _currentsongindex 1)
    (`KismetSystemLibrary.K2_SetTimer` null "MorzeSignal" 60.0))
  (if (== (`KismetArrayLibrary.Array_LastIndex` _songslist) _currentsongindex)
    (set `self.CurrentSongIndex` 0)
    (else
      (`/Engine/EditorBlueprintResources/StandardMacros.IncrementInt` _currentsongindex))))

(fn `MorzeSignal`
  (bind _audio (`self.Audio`))
  (set `AudioComponent.Sound` "/Game/Sounds/Unsort/CUE_WHITESPACE_morse.CUE_WHITESPACE_morse" _audio)
  (`AudioComponent.Play` _audio 0.0))

(fn `UserConstructionScript`)