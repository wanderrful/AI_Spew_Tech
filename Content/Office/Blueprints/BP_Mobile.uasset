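; BP_Mobile is a usable phone prop that receives a secret text message some minutes after play begins.
; A one-shot timer started at BeginPlay flags the arrival and starts a looping RingCell timer that repeats the new-message text and ring sound.
; OnUse before arrival shows "No Messages" briefly.
; The first use after arrival reveals SMSSecret and stops the ringing, and later uses do nothing.
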(event `self.OnUse`
  (bind _screentext (`self.ScreenText`))
  (if (`self.SMSBeenRead`)
    _
    (elif (`self.SMSHasArrived`)
      (`TextRenderComponent.K2_SetText` _screentext (`self.SMSSecret`))
      (`KismetSystemLibrary.K2_ClearTimer` null "RingCell")
      (set `self.SMSBeenRead` true)
      (`AudioComponent.Stop` (`self.CellRingSound`))
      (else
        (`TextRenderComponent.K2_SetText` _screentext (`KismetTextLibrary.Conv_StringToText` "No Messages"))
        (`KismetSystemLibrary.K2_SetTimer` null "TurnOff" 15.0)))))

(event `self.ReceiveBeginPlay`
  (`KismetSystemLibrary.K2_SetTimerDelegate` (delegate `SMSArrived`) 300.0))

(event `SMSArrived`
  (set `self.SMSHasArrived` true)
  (`KismetSystemLibrary.K2_SetTimer` null "RingCell" 10.0 true)
  (`KismetSystemLibrary.K2_ClearTimer` null "TurnOff"))

(fn `RingCell`
  (bind _cellringsound (`self.CellRingSound`))
  (`TextRenderComponent.K2_SetText` (`self.ScreenText`) (`KismetTextLibrary.Conv_StringToText` "New Message!"))
  (`AudioComponent.SetSound` _cellringsound "/Game/Sounds/ShortSounds/A_CellRing.A_CellRing")
  (`AudioComponent.Play` _cellringsound 0.0))

(fn `TurnOff`
  (`TextRenderComponent.K2_SetText` (`self.ScreenText`) (`KismetTextLibrary.Conv_StringToText` "")))

(fn `UserConstructionScript`)