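; BP_FluorescentLight is an office fluorescent light that flickers at random intervals during play.
; On BeginPlay it stores the light's starting intensity and sets a one-shot timer with a random delay.
; Each blink plays a sound and runs a timeline curve that scales the starting intensity, then schedules the next blink with a new random delay.
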(event `self.ReceiveBeginPlay`
  (set `self.StartBrightness` (`LightComponentBase.Intensity` (`self.LightComponent0`)))
  (`KismetSystemLibrary.K2_SetTimerDelegate` (delegate `Blink`) (* (+ (`KismetMathLibrary.RandomFloat`) 1.0) 10.0)))

(event `Blink`
  (`AudioComponent.Play` (`self.Audio`) 0.0)
  (bind (_direction _blinkbrightness) (`Timeline|BlinkCurve` :!via `PlayFromStart`)
    (:`Update`
      (`LightComponent.SetIntensity` (`self.LightComponent0`) (* _blinkbrightness (`self.StartBrightness`))))
    (:`Finished`
      (`KismetSystemLibrary.K2_SetTimerDelegate` (delegate `Blink`) (* (+ (`KismetMathLibrary.RandomFloat`) 1.0) 10.0)))))

(fn `UserConstructionScript`)